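; BP_SkvtScreen is a screen actor that displays a WBP_SkvtWeb widget and can be turned on, turned off or broken.
; On BeginPlay it caches the widget from its Webpage component and calls UpdateScreen with false.
; Turnon, TurnOff and Shorten route through ToggleScreen, which sets the widget's IsOn and calls its matching function.
; Shorten also sets IsCrashed, which blocks any later Turnon since nothing here clears it.
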(event `self.ReceiveBeginPlay`
  (`self.Initialize`))

(event `/Game/Skvt/Blueprints/BPI_Electronics.TurnOn`
  (if (not (`self.IsCrashed`))
    (`self.ToggleScreen` true)))

(event `/Game/Skvt/Blueprints/BPI_Electronics.TurnOff`
  (`self.ToggleScreen` false))

(event `/Game/Skvt/Blueprints/BPI_Electronics.Shorten`
  (`self.ToggleScreen` false)
  (set `self.IsCrashed` true))

(fn `Initialize`
  (bind _aswbp_skvt_web (cast `/Game/Skvt/Blueprints/Screen/WBP_SkvtWeb` (`WidgetComponent.GetWidget` (`self.Webpage`))))
  (bind _output_get (set `self.WebpageRef` _aswbp_skvt_web))
  (`/Game/Skvt/Blueprints/Screen/WBP_SkvtWeb.UpdateScreen` _output_get false))

(fn `ToggleScreen`
  (params (IsOn :type Boolean))
  (bind _webpageref (`self.WebpageRef`))
  (bind _output_get (set `/Game/Skvt/Blueprints/Screen/WBP_SkvtWeb.IsOn` IsOn _webpageref))
  (if _output_get
    (`/Game/Skvt/Blueprints/Screen/WBP_SkvtWeb.TurnOn` _webpageref)
    (else
      (`/Game/Skvt/Blueprints/Screen/WBP_SkvtWeb.TurnOff` _webpageref))))

(fn `UserConstructionScript`)