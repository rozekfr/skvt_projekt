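; Blueprint function library with an EMP pulse that hits electronics around a given actor.
; EMPImpuls gathers every actor implementing BPI_Electronics and keeps those within the source actor's Radius, measured in 2D so height is ignored.
; Each one in range receives the ShortenMessage interface call, then smoke and spark emitters and an explosion sound spawn at its location.
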(fn `EMPImpuls`
  (params (Actor :type "/Game/Skvt/Blueprints/Platform/BP_EMPPlatform Object Reference"))
  (bind _outactors (`GameplayStatics.GetAllActorsWithInterface` null "/Game/Skvt/Blueprints/BPI_Electronics.BPI_Electronics_C"))
  (for _array_element _outactors
    (bind _returnvalue (`Actor.K2_GetActorLocation` _array_element))
    (if (<= (`KismetMathLibrary.Vector_Distance2D` _returnvalue (`Actor.K2_GetActorLocation` Actor)) (`/Game/Skvt/Blueprints/Platform/BP_EMPPlatform.Radius` Actor))
      (message `/Game/Skvt/Blueprints/BPI_Electronics.Shorten` _array_element)
      (`GameplayStatics.SpawnEmitterAtLocation` null "/Game/StarterContent/Particles/P_Smoke.P_Smoke" _returnvalue)
      (`GameplayStatics.SpawnEmitterAtLocation` null "/Game/StarterContent/Particles/P_Sparks.P_Sparks" _returnvalue)
      (`GameplayStatics.SpawnSoundAtLocation` null "/Game/StarterContent/Audio/Explosion_Cue.Explosion_Cue" _returnvalue (struct) 1.0 1.0 0.0 null null))))