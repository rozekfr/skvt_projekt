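; BP_TogglePlatform is a platform that switches linked electronics on while an actor overlaps it and off when an overlap ends.
; Overlap events pass the state to ToggleElectronics, which sends TurnOn or TurnOff messages to each entry in the Electronics array.
; Overlaps are neither filtered nor counted, so any actor leaving turns everything off.
; ToggleLights does the same for the Lights array but is not called in this Blueprint.
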(event `self.ReceiveActorBeginOverlap`
  (params (OtherActor :type "Actor Object Reference"))
  (`self.ToggleElectronics` true))

(event `self.ReceiveActorEndOverlap`
  (params (OtherActor :type "Actor Object Reference"))
  (`self.ToggleElectronics` false))

(fn `ToggleElectronics`
  (params (IsOn :type Boolean))
  (for _array_element (`self.Electronics`)
    (if IsOn
      (message `/Game/Skvt/Blueprints/BPI_Electronics.TurnOn` _array_element)
      (else
        (message `/Game/Skvt/Blueprints/BPI_Electronics.TurnOff` _array_element)))))

(fn `ToggleLights`
  (params (TurnOn :type Boolean))
  (for _array_element (`self.Lights`)
    (`/Game/Skvt/Blueprints/Light/BP_WallSconce.Toggle Light` _array_element TurnOn)))

(fn `UserConstructionScript`)