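; BP_EMPPlatform is a platform that sets off an EMP impulse the first time an actor overlaps it.
; The overlap event calls EMPImpuls, whose body is not shown here, then sets IsTriggered so later overlaps do nothing.
; The construction script draws a temporary debug sphere at the actor's location to visualize its Radius.
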(event `self.ReceiveBeginPlay`)

(event `self.ReceiveActorBeginOverlap`
  (params (OtherActor :type "Actor Object Reference"))
  (if (not (`self.IsTriggered`))
    (`/Game/Skvt/Blueprints/Platform/BFL_EMP.EMPImpuls` self)
    (set `self.IsTriggered` true)))

(event `self.ReceiveActorEndOverlap`
  (params (OtherActor :type "Actor Object Reference")))

(fn `UserConstructionScript`
  (`KismetSystemLibrary.DrawDebugSphere` (`self.K2_GetActorLocation`) (`self.Radius`) 12 (struct :`R` 1.0 :`G` 1.0 :`B` 1.0 :`A` 1.0) 10.0 1.0))