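; Player controller for the Skvt game that lets the player swap between the male and female characters and toggle a pausing main menu.
; BeginPlay creates the HUD for the local player and adds default and pawn-swap Enhanced Input mapping contexts.
; Swap input possesses the opposite character found by class lookup, while menu input creates or removes the menu widget, switching input mode, cursor and pause.
; UpdateHealthBar forwards a health bar component to the HUD.
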(event `self.ReceiveBeginPlay`
  (bind _returnvalue (pcsubsystem `EnhancedInputLocalPlayerSubsystem` self))
  (`self.SpawnHUD`)
  (`/Engine/EditorBlueprintResources/StandardMacros.IsValid` _returnvalue
    (:`Is Valid`
      (`EnhancedInputSubsystemInterface.AddMappingContext` _returnvalue "/Game/ThirdPerson/Input/IMC_Default.IMC_Default" 0 (struct))
      (`EnhancedInputSubsystemInterface.AddMappingContext` _returnvalue "/Game/Skvt/Characters/Input/IMC_SwapPawn.IMC_SwapPawn" 0 (struct)))))

(event `EnhancedInput|/Game/Skvt/Characters/Input/Actions/IA_Swap`
  (params (ActionValue :type Boolean) (ElapsedSeconds :type "Float (double-precision)") (TriggeredSeconds :type "Float (double-precision)") (InputAction :type "InputAction Object Reference" :default "/Game/Skvt/Characters/Input/Actions/IA_Swap.IA_Swap"))
  (:`Triggered`
    (if (`.bSuccess` (cast `/Game/Skvt/Characters/BP_SkvtCharacterFemale` (`GameplayStatics.GetPlayerPawn` 0) :!pure true))
      (bind _returnvalue (`GameplayStatics.GetActorOfClass` "/Game/Skvt/Characters/BP_SkvtCharacterMale.BP_SkvtCharacterMale_C"))
      (`self.Possess` _returnvalue)
      (else
        (bind _returnvalue_2 (`GameplayStatics.GetActorOfClass` "/Game/Skvt/Characters/BP_SkvtCharacterFemale.BP_SkvtCharacterFemale_C"))
        (`self.Possess` _returnvalue_2)))))

(event `EnhancedInput|/Game/Skvt/Characters/Input/Actions/IA_OpenMenu`
  (params (ActionValue :type Boolean) (ElapsedSeconds :type "Float (double-precision)") (TriggeredSeconds :type "Float (double-precision)") (InputAction :type "InputAction Object Reference" :default "/Game/Skvt/Characters/Input/Actions/IA_OpenMenu.IA_OpenMenu"))
  (:`Triggered`
    (if (`self.IsMainMenuOpen`)
      (`self.CloseMainMenu`)
      (else
        (`self.OpenMainMenu`)))))

(fn `CloseMainMenu`
  (`Widget.RemoveFromParent` (`self.MainMenuRef`))
  (set `self.MainMenuRef` null)
  (`WidgetBlueprintLibrary.SetInputMode_GameOnly` self)
  (set `self.bShowMouseCursor` false)
  (`GameplayStatics.SetGamePaused` false))

(fn `IsMainMenuOpen`
  (returns (IsOpen :type Boolean))
  (return (`KismetSystemLibrary.IsValid` (`self.MainMenuRef`))))

(fn `OpenMainMenu`
  (bind _returnvalue (`|CreateWidget` "/Game/Skvt/UI/Widgets/Menu/WBP_MainMenu.WBP_MainMenu_C" self))
  (bind _output_get (set `self.MainMenuRef` _returnvalue))
  (`UserWidget.AddToViewport` _output_get 0)
  (set `self.bShowMouseCursor` true)
  (`GameplayStatics.SetGamePaused` true)
  (`WidgetBlueprintLibrary.SetInputMode_GameAndUIEx` self null))

(fn `SpawnHUD`
  (if (`self.IsLocalPlayerController`)
    (bind _returnvalue (`|CreateWidget` "/Game/Skvt/UI/Widgets/HUD/WBP_HUD.WBP_HUD_C" self))
    (bind _output_get (set `self.HUDRef` _returnvalue))
    (`UserWidget.AddToViewport` _output_get 0)))

(fn `UpdateHealthBar`
  (params (NewHealthBarComponent :type "/Game/Skvt/Systems/DamageSystem/SkvtHealthComponent Object Reference"))
  (`/Game/Skvt/UI/Widgets/HUD/WBP_HUD.InitializeHealthBar` (`self.HUDRef`) NewHealthBarComponent))

(fn `UserConstructionScript`)