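; Base NPC Blueprint that, going by its name, underpins behavior-tree-driven NPCs by feeding sight detection into the AI.
; When its PawnSensing component sees a pawn, it sets the controller's blackboard bool named by the SeenPlayerName variable to true.
; The handler neither checks that the seen pawn is the player nor clears the flag, and no other event has active logic.
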(event `self.PawnSensing.OnSeePawn`
  (params (Pawn :type "Pawn Object Reference"))
  (`BlackboardComponent.SetValueAsBool` (`AIBlueprintHelperLibrary.GetBlackboard` (`self.GetController`)) (`self.SeenPlayerName`) true))

(fn `UserConstructionScript`
  (`parent.UserConstructionScript`))