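; Base NPC character that takes damage, attacks and dies, delegating damage and attack logic to its SkvtHealthComponent.
; Incoming damage is passed to the component and plays a punch hit-reaction montage.
; On death, the mesh simulates physics, movement is disabled and a timer destroys the actor after a short delay.
; Attack hands the component the world locations of the AttackStart and AttackEnd points.
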(event `self.SkvtHealthComponent.OnDeath`
  (`PrimitiveComponent.SetSimulatePhysics` (`self.Mesh`) true)
  (`CharacterMovementComponent.DisableMovement` (`self.CharacterMovement`))
  (`KismetSystemLibrary.K2_SetTimerDelegate` (delegate `FinalizeDeath`) 5.0))

(event `FinalizeDeath`
  (`self.K2_DestroyActor`))

(event `self.ReceiveAnyDamage`
  (params (Damage :type "Float (single-precision)") (DamageType :type "DamageType Object Reference") (InstigatedBy :type "Controller Object Reference") (DamageCauser :type "Actor Object Reference"))
  (`/Game/Skvt/Systems/DamageSystem/SkvtHealthComponent.ProcessDamage` (`self.SkvtHealthComponent`) Damage)
  (`self.PlayAnimMontage` "/Game/Skvt/Characters/Animations/Attacks/AM_Hit_punch.AM_Hit_punch"))

(fn `Attack`
  (`/Game/Skvt/Systems/DamageSystem/SkvtHealthComponent.Attack` (`self.SkvtHealthComponent`) (`SceneComponent.K2_GetComponentLocation` (`self.AttackStart`)) (`SceneComponent.K2_GetComponentLocation` (`self.AttackEnd`))))

(fn `UserConstructionScript`)